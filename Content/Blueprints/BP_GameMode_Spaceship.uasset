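; Game mode for a spaceship game that tracks total wins and losses and handles the end screen and restarts.
; CE_Bind hooks the player pawn's game-over and game-won dispatchers to events that increment the matching counter and show an EndScreen widget flagged as win or loss.
; CE_RestartGame destroys the pawn, waits briefly, spawns a new one at the PlayerStart, then tells BP_EnemyController to spawn enemies again.
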(event `CE_Bind`
  (bind _playerpawnref (`self.PlayerPawnRef`))
  (add `/Game/Blueprints/BP_PlayerPawn.ED_GameOver` _playerpawnref (delegate `CE_ShowEndgameScreen`))
  (add `/Game/Blueprints/BP_PlayerPawn.ED_GameWon` _playerpawnref (delegate `CE_GameWon`)))

(event `CE_ShowEndgameScreen`
  (`/Engine/EditorBlueprintResources/StandardMacros.IncrementInt` (`self.TotalLoses`)
    (:`  `
      (bind _returnvalue (`|CreateWidget` "/Game/Blueprints/EndScreen.EndScreen_C"))
      (`UserWidget.AddToViewport` _returnvalue 0))))

(event `CE_GameWon`
  (`/Engine/EditorBlueprintResources/StandardMacros.IncrementInt` (`self.TotalWins`)
    (:`  `
      (bind _returnvalue (`|CreateWidget` "/Game/Blueprints/EndScreen.EndScreen_C" null true))
      (`UserWidget.AddToViewport` _returnvalue 0))))

(event `CE_RestartGame`
  (`self.K2_DestroyActor` (`self.PlayerPawnRef`))
  (`KismetSystemLibrary.Delay` 0.05)
  (bind _returnvalue (`GameplayStatics.GetActorOfClass` "/Script/Engine.PlayerStart"))
  (`|SpawnActorFromClass` "/Game/Blueprints/BP_PlayerPawn.BP_PlayerPawn_C" (`self.GetTransform` _returnvalue) "Undefined" "MultiplyWithRoot" null null)
  (bind _returnvalue_2 (`GameplayStatics.GetActorOfClass` "/Game/Blueprints/BP_EnemyController.BP_EnemyController_C"))
  (`/Game/Blueprints/BP_EnemyController.CE_SpawnEnemy` _returnvalue_2))

(fn `UserConstructionScript`)