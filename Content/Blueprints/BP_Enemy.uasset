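; Enemy actor that fires green bullets at the player and asks its owning BP_EnemyController for a replacement when destroyed.
; A looping timeline eases CurrentHeight toward a fixed value, then re-randomizes it.
; Shots aim with random vertical spread that narrows as Health drops, while hits hide health-bar images until the enemy dies.
; Player game-over or win events destroy it without respawn or explosion sound.
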(event `self.ReceiveBeginPlay`
  (add `self.OnDestroyed` (delegate `OnDestroyed_Event`))
  (bind _asbp_player_pawn (cast `/Game/Blueprints/BP_PlayerPawn` (`self.PlayerPawn`)))
  (add `/Game/Blueprints/BP_PlayerPawn.ED_GameOver` _asbp_player_pawn (delegate `CE_GameOver`))
  (add `/Game/Blueprints/BP_PlayerPawn.ED_GameWon` _asbp_player_pawn (delegate `CE_GameWon`))
  (`Timeline|Timeline_PositionChange` :!label _label
    (:`Update`
      (set `self.CurrentHeight` (`KismetMathLibrary.Lerp` (`self.CurrentHeight`) 20.0 (/ (`TimelineComponent.GetPlaybackPosition` (`self.Timeline_PositionChange`)) 5.0))))
    (:`Finished`
      (set `self.CurrentHeight` (`KismetMathLibrary.RandomFloatInRange` -500.0 500.0))
      (goto _label :!via `PlayFromStart`))))

(event `CE_GameOver`
  (`self.SetActorTickEnabled` false :!label _label_2)
  (set `self.isEndGame` true)
  (`self.K2_DestroyActor`))

(event `OnDestroyed_Event` :!signature `self.OnDestroyed`
  (params (DestroyedActor :type "Actor Object Reference"))
  (if (not (`self.isEndGame`))
    (bind _asbp_enemy_controller (cast `/Game/Blueprints/BP_EnemyController` (`self.GetOwner`)))
    (`/Game/Blueprints/BP_EnemyController.CE_SpawnEnemy` _asbp_enemy_controller)
    (`GameplayStatics.PlaySound2D` "/Game/SFX/explosion.explosion" 1.0 1.0 0.0 null null)))

(event `CE_GameWon`
  (goto _label_2))

(event `self.Shoot`
  (bind _health (`self.Health`))
  (bind _returnvalue (+ (`self.K2_GetActorLocation`) (0.0 -120.0 -20.0)))
  (bind (_returnvalue_roll _returnvalue_pitch _returnvalue_yaw) (`KismetMathLibrary.BreakRotator` (`KismetMathLibrary.FindLookAtRotation` _returnvalue (+ (`self.K2_GetActorLocation` (`self.PlayerPawn`)) (`KismetMathLibrary.MakeVector` 0.0 0.0 (`KismetMathLibrary.RandomFloatInRange` (select `int` _health :`0` 0.0 :`1` -120.0 :`2` -130.0 :`3` -150.0) (select `int` _health :`0` 0.0 :`1` 120.0 :`2` 130.0 :`3` 150.0)))))))
  ;[1 1 1] Shoot
  (`|SpawnActorFromClass` "/Game/Blueprints/BP_Bullet.BP_Bullet_C" (`KismetMathLibrary.MakeTransform` _returnvalue (`KismetMathLibrary.MakeRotator` _returnvalue_roll _returnvalue_pitch _returnvalue_yaw)) "Undefined" "MultiplyWithRoot" null "Green" null))

(event `CE_Damage`
  (bind _health (`self.Health`))
  ;[1 1 1] Damage
  (if (> _health 1)
    (`self.Damage`)
    (bind _asbp_enemy_health_bar (cast `/Game/Blueprints/BP_EnemyHealthBar` (`WidgetComponent.GetWidget` (`self.Widget`))))
    (`Widget.SetVisibility` (select `int` _health :`0` (`/Game/Blueprints/BP_EnemyHealthBar.Image_0` _asbp_enemy_health_bar) :`1` (`/Game/Blueprints/BP_EnemyHealthBar.Image_1` _asbp_enemy_health_bar) :`2` (`/Game/Blueprints/BP_EnemyHealthBar.Image_2` _asbp_enemy_health_bar) :!type "Widget Object Reference") "Hidden")
    (`GameplayStatics.PlaySound2D` "/Game/SFX/hit.hit" 1.0 1.0 0.0 null null)
    (else
      (`self.K2_DestroyActor`))))

(fn `UserConstructionScript`)