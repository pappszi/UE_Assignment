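; BP_Bullet is a projectile whose BulletColor decides both its look and whom it damages.
; On spawn it plays a laser sound, with pitch chosen by color.
; When its Cylinder overlaps an actor, a red bullet damages only BP_Enemy and other colors only BP_PlayerPawn, destroying itself on a hit.
; The construction script tints green bullets through a dynamic material instance.
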(event `self.ReceiveBeginPlay`
  (`GameplayStatics.PlaySound2D` "/Game/SFX/Laser.Laser" 1.0 (select `byte` (`self.BulletColor`) :`0` 1.0 :`1` 0.7 :!type "Float (single-precision)") 0.0 null null))

(event `self.Cylinder.OnComponentBeginOverlap`
  (params (OverlappedComponent :type "PrimitiveComponent Object Reference") (OtherActor :type "Actor Object Reference") (OtherComp :type "PrimitiveComponent Object Reference") (OtherBodyIndex :type Integer) (bFromSweep :type Boolean) (SweepResult :type "HitResult Structure (by ref)"))
  (if (`|EnumEquality` (`self.BulletColor`) "Red")
    (bind _asbp_enemy (cast `/Game/Blueprints/BP_Enemy` OtherActor))
    (`/Game/Blueprints/BP_Enemy.CE_Damage` _asbp_enemy)
    (`self.K2_DestroyActor`)
    (else
      (bind _asbp_player_pawn (cast `/Game/Blueprints/BP_PlayerPawn` OtherActor))
      (`/Game/Blueprints/BP_PlayerPawn.CE_Damage` _asbp_player_pawn)
      (`self.K2_DestroyActor`))))

(fn `UserConstructionScript`
  (if (`|EnumEquality` (`self.BulletColor`) "Green")
    (bind _returnvalue (`PrimitiveComponent.CreateDynamicMaterialInstance` (`self.Cylinder`) 0 "/Game/Materials/M_Bullet_Inst.M_Bullet_Inst" "None"))
    (`MaterialInstanceDynamic.SetVectorParameterValue` _returnvalue "Color" (struct :`G` 10.0 :`A` 1.0))))