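; BP_FloatingIsland is an actor that makes an island bob gently up and down in place.
; BeginPlay stores the starting location and picks a random phase offset.
; Tick sets the height from a sine of game-state time plus that offset, so separate islands move out of sync while oscillating around their placed position.
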(event `self.ReceiveBeginPlay`
  (set `self.RandomStartDelay` (`KismetMathLibrary.RandomFloatInRange` -1.0 1.0))
  (set `self.InitialLocation` (`self.K2_GetActorLocation`)))

(event `self.ReceiveTick`
  (params (DeltaSeconds :type "Float (single-precision)"))
  (`self.K2_SetActorLocation` (+ (`self.InitialLocation`) (`KismetMathLibrary.MakeVector` 0.0 0.0 (* (`KismetMathLibrary.Sin` (+ (/ (`self.GetGameTimeSinceCreation` (`GameplayStatics.GetGameState`)) 2.0) (`self.RandomStartDelay`))) 180.0)))))

(fn `UserConstructionScript`)