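; Player pawn for a spaceship shooter, with input-driven movement, mouse-crosshair shooting and health.
; Movement input is clamped against overlapped invisible walls, and shots take rotation from a fixed screen reference point to the cursor, gated by a cooldown shown on the HUD.
; Damage updates a widget health bar and either restarts delayed step-by-step regeneration or triggers game over.
; It registers with the spaceship game mode, disabling input and tick on win or loss.
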(event `self.ReceiveBeginPlay`
  (bind _returnvalue (`GameplayStatics.GetPlayerController` 0))
  ;[1 1 1] BeginPlay
  (`EnhancedInputSubsystemInterface.AddMappingContext` (pcsubsystem `EnhancedInputLocalPlayerSubsystem` _returnvalue) "/Game/ThirdPerson/Input/IMC_Default.IMC_Default" 0 (struct))
  (set `PlayerController.bShowMouseCursor` true _returnvalue)
  (bind _returnvalue_2 (`|CreateWidget` "/Game/Blueprints/BP_Crosshair.BP_Crosshair_C"))
  (`PlayerController.SetMouseCursorWidget` _returnvalue "Default" _returnvalue_2)
  (bind _asbp_game_mode_spaceship (cast `/Game/Blueprints/BP_GameMode_Spaceship` (`GameplayStatics.GetGameMode`)))
  (set `/Game/Blueprints/BP_GameMode_Spaceship.PlayerPawnRef` self _asbp_game_mode_spaceship)
  (`/Game/Blueprints/BP_GameMode_Spaceship.CE_Bind` _asbp_game_mode_spaceship)
  (add `self.ED_GameOver` (delegate `CE_GameOver`))
  (add `self.ED_GameWon` (delegate `CE_GameWon`)))

(event `CE_GameWon`
  (`self.DisableInput` (`GameplayStatics.GetPlayerController` 0) :!label _label)
  (`self.SetActorTickEnabled` false)
  (set `PrimitiveComponent.bGenerateOverlapEvents` false (`self.SkeletalMesh`)))

(event `CE_GameOver`
  (goto _label))

(event `EnhancedInput|/Game/ThirdPerson/Input/Actions/IA_Move`
  (params (ActionValue :type "Vector2D Structure") (ElapsedSeconds :type "Float (double-precision)") (TriggeredSeconds :type "Float (double-precision)") (InputAction :type "InputAction Object Reference" :default "/Game/ThirdPerson/Input/Actions/IA_Move.IA_Move"))
  (bind _overlappingactors (`self.GetOverlappingActors` "/Game/Blueprints/BP_InvisibleWall.BP_InvisibleWall_C"))
  ;[1 1 1] Move
  (:`Triggered`
    (if (> (`KismetArrayLibrary.Array_Length` _overlappingactors) 0)
      (bind _constrainedinput (`self.CheckNavigateConstraint` _overlappingactors ActionValue))
      (`self.NavigatePlayer` _constrainedinput 400.0)
      (else
        (`self.NavigatePlayer` ActionValue 400.0))))
  (:`Completed`
    (set `self.bShouldAscend` true)))

(event `self.GameWon`
  (`self.ED_GameWon`))

(event `EnhancedInput|/Game/ThirdPerson/Input/Actions/IA_Shoot`
  (params (ActionValue :type Boolean) (ElapsedSeconds :type "Float (double-precision)") (TriggeredSeconds :type "Float (double-precision)") (InputAction :type "InputAction Object Reference" :default "/Game/ThirdPerson/Input/Actions/IA_Shoot.IA_Shoot"))
  (bind (_locationx _locationy) (`WidgetLayoutLibrary.GetMousePositionScaledByDPI` (`GameplayStatics.GetPlayerController` 0)))
  (bind (_returnvalue_roll _returnvalue_pitch _returnvalue_yaw) (`KismetMathLibrary.BreakRotator` (`KismetMathLibrary.FindLookAtRotation` (`KismetMathLibrary.MakeVector` 0.0 900.0 500.0) (`KismetMathLibrary.MakeVector` 0.0 _locationx _locationy))))
  ;[1 1 1] Shoot
  (:`Started`
    (`/Engine/EditorBlueprintResources/StandardMacros.Gate` false :!label _label_2
      (:`Exit`
        (`|SpawnActorFromClass` "/Game/Blueprints/BP_Bullet.BP_Bullet_C" (`KismetMathLibrary.MakeTransform` (+ (`self.K2_GetActorLocation`) (-40.0 0.0 70.0)) (`KismetMathLibrary.MakeRotator` _returnvalue_roll (* _returnvalue_pitch -1.0) _returnvalue_yaw)) "Undefined" "MultiplyWithRoot" null "Red" self)
        (bind _asbp_hud (cast `/Game/Blueprints/BP_HUD` (`PlayerController.GetHUD` (`GameplayStatics.GetPlayerController` 0)))
          (:`then`
            (`TimelineComponent.PlayFromStart` (`/Game/Blueprints/BP_HUD.Timeline_ShootCooldown` _asbp_hud)))
          (:`CastFailed`
            _))
        (`|ExecutionSequence`
          (:`then_0`
            (cast `/Game/Blueprints/BP_PlayerHealthBar` (`WidgetComponent.GetWidget` (`self.Widget`)))
            (goto _label_2 :!via `Close`))
          (:`then_1`
            (`KismetSystemLibrary.Delay` 1.0)
            (goto _label_2 :!via `Open`)))))))

(event `CE_Damage`
  (bind _health (`self.Health`))
  ;[1 1 1] TakeDamage
  (`self.SetHealth` (- _health 1))
  (bind _asbp_player_health_bar (cast `/Game/Blueprints/BP_PlayerHealthBar` (`WidgetComponent.GetWidget` (`self.Widget`))))
  (`/Game/Blueprints/BP_PlayerHealthBar.CE_DeacreaseHealth` _asbp_player_health_bar _health)
  (if (> _health 0)
    (`self.CE_HealthRegenStart`)
    (`GameplayStatics.PlaySound2D` "/Game/SFX/hit.hit" 1.0 0.5 0.0 null null)
    (else
      (`self.ED_GameOver`))))

(event `CE_HealthRegenStart`
  ;[1 1 1] Start Health Regen
  (`KismetSystemLibrary.RetriggerableDelay` 2.0)
  (if (!= (`self.Health`) 0)
    (`self.CE_HealthRegen`)))

(event `CE_HealthRegen`
  (bind _health (`self.Health`))
  ;[1 1 1] HealthRegen
  (if (!= _health 6)
    (bind _asbp_player_health_bar (cast `/Game/Blueprints/BP_PlayerHealthBar` (`WidgetComponent.GetWidget` (`self.Widget`))))
    (`/Game/Blueprints/BP_PlayerHealthBar.CE_IncreaseHealth` _asbp_player_health_bar _health)
    (`self.SetHealth` (+ _health 1))
    (if (< (`self.Health`) 6)
      (`self.CE_HealthRegenStart`))))

(fn `CheckNavigateConstraint`
  (params (InvisibleWall :type "Array of Actor Object Reference (by ref)") (InputVec :type "Vector2D Structure (by ref)"))
  (returns (ConstrainedInput :type "Vector2D Structure"))
  (locals (InputOut :type "Vector2D Structure" :default (0.0 0.0)))
  (bind (_x _y) (`KismetMathLibrary.BreakVector2D` InputVec))
  (for (_array_element _array_index) InvisibleWall
    (bind _asbp_invisible_wall (cast `/Game/Blueprints/BP_InvisibleWall` _array_element))
    (if (== _array_index 0)
      (bind _returnvalue (select `/Game/Blueprints/E_WallPosition` (`/Game/Blueprints/BP_InvisibleWall.Wallposition` _asbp_invisible_wall) :`NewEnumerator0` (`KismetMathLibrary.MakeVector2D` (`KismetMathLibrary.FClamp` _x) _y) :`NewEnumerator1` (`KismetMathLibrary.MakeVector2D` (`KismetMathLibrary.FClamp` _x -1.0 0.0) _y) :`NewEnumerator3` (`KismetMathLibrary.MakeVector2D` _x (`KismetMathLibrary.FClamp` _y))))
      (set `local.InputOut` _returnvalue)
      (else
        (set `local.InputOut` (* (`local.InputOut`) _returnvalue)))))
  (return (`local.InputOut`)))

(fn `UserConstructionScript`)